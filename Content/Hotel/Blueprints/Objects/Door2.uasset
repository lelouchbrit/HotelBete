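; Locked hotel door that swings open on its hinge when the player unlocks it with a key, as the second step in a door sequence.
; OpenDoor requires the player's DoorCount to equal one and a KEY in InventoryB, then consumes the key, increments the count and sets IsOpened.
; Tick treats IsOpened as a one-shot trigger, clearing it and starting an eased MoveComponentTo rotation, so DoorCount alone prevents reopening.
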(event EventBeginPlay)

(event Collision|EventActorBeginOverlap
  (params (OtherActor :type Actor%20Object%20Reference)))

(event EventTick
  (params (DeltaSeconds :type Float%20%28single-precision%29))
  (bind _hinge (Variables|Default|GetHinge))
  (if (Variables|Default|GetIsOpened)
    (Variables|Default|SetIsOpened false)
    (Components|MoveComponentTo _hinge (Variables|/Script/Engine.SceneComponent|GetRelativeLocation _hinge) "0,-90.000000, 0" true true 0.7)))

(fn ConstructionScript)

(fn OpenDoor
  (bind _stuffa (Utilities|Struct|MakeStuffA "KEY" "/Game/FirstPersonBP/Textures/KeyPic.KeyPic"))
  (if (not (Variables|Default|GetIsOpened))
    (Development|PrintString "Hello1")
    (bind _asplayer (Utilities|Casting|CastToPlayer (Game|GetPlayerCharacter 0)))
    (Math|Float|CompareFloat (Variables|/Game/Hotel/Blueprints/Player/Player.Player_C|GetDoorCount _asplayer) 1.0
      (:==
        (Development|PrintString "Hello2")
        (if (Utilities|Array|ContainsItem (Variables|/Game/Hotel/Blueprints/Player/Player.Player_C|GetInventoryB _asplayer) _stuffa)
          (Utilities|Array|RemoveItem (Variables|/Game/Hotel/Blueprints/Player/Player.Player_C|GetInventoryB _asplayer) _stuffa)
          (Variables|Default|SetIsOpened true)
          (bind _output_get (Variables|/Game/Hotel/Blueprints/Player/Player.Player_C|SetDoorCount _asplayer (+ (Variables|/Game/Hotel/Blueprints/Player/Player.Player_C|GetDoorCount _asplayer) 1.0)))
          (Development|PrintString (Utilities|String|ToString(Float) _output_get)))))))