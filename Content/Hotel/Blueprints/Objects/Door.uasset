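; Locked hotel door that opens when the player overlaps its box while carrying a key.
; OpenDoor finds player 0's KEY entry in InventoryB by matching a rebuilt item struct, name and picture included, then removes it.
; The door opens instantly by moving and yawing the whole actor from the Hinge's world transform, with no animation.
; An unconnected DestroyActor call never runs.
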(event OnComponentBeginOverlap(Box)
  (params (OtherActor :type Actor%20Object%20Reference) (OtherComp :type Primitive%20Component%20Object%20Reference) (OtherBodyIndex :type Integer) (bFromSweep :type Boolean) (SweepResult :type Hit%20Result%20Structure%20%28by%20ref%29))
  (Utilities|Casting|CastToPlayer OtherActor)
  (CallFunction|OpenDoor))

(event EventBeginPlay)

(event EventActorBeginOverlap
  (params (OtherActor :type Actor%20Object%20Reference)))

(event EventTick
  (params (DeltaSeconds :type Float%20%28single-precision%29)))

(fn ConstructionScript)

(fn OpenDoor
  (bind _stuffa (Utilities|Struct|MakeStuffA "KEY" "/Game/Hotel/Art/Textures/Lobby/Ceiling/Ceiling_Base_Color.Ceiling_Base_Color"))
  (bind _hinge (Variables|Default|GetHinge))
  (bind _returnvalue (Transformation|GetWorldLocation _hinge))
  (bind _returnvalue_2 (Transformation|GetWorldRotation _hinge))
  (bind (_x _y _z) (Math|Vector|BreakVector _returnvalue))
  (bind (_roll _pitch _yaw) (Math|Rotator|BreakRotator _returnvalue_2))
  (bind _asplayer (Utilities|Casting|CastToPlayer (Game|GetPlayerCharacter 0)))
  (if (Utilities|Array|ContainsItem (Variables|/Game/Hotel/Blueprints/Player/Player.Player_C|GetInventoryB _asplayer) _stuffa)
    (Utilities|Array|RemoveItem (Variables|/Game/Hotel/Blueprints/Player/Player.Player_C|GetInventoryB _asplayer) _stuffa)
    (Transformation|SetActorLocationAndRotation (Math|Vector|MakeVector (+ _x 7e+01) _y _z) (Math|Rotator|MakeRotator _roll _pitch (+ _yaw -9e+01)))))