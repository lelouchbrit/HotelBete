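; Hotel enemy that frightens the player by proximity and is destroyed when a camera-shot projectile overlaps its CamTarget.
; Every tick it hides its sphere while the player's camera is up and shows it otherwise.
; When the player is close, it also raises SpookLevel by inverse distance each frame, so the gain is framerate-dependent.
; Destruction stops the player's heartbeat, while pawn sensing and AI perception only print debug names.
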(event OnTargetPerceptionUpdated(AIPerception)
  (params (Actor :type Actor%20Object%20Reference) (Stimulus :type AI%20Stimulus%20Structure))
  (Development|PrintString (Utilities|GetDisplayName Actor)))

(event OnComponentBeginOverlap(CamTarget)
  (params (OtherActor :type Actor%20Object%20Reference) (OtherComp :type Primitive%20Component%20Object%20Reference) (OtherBodyIndex :type Integer) (bFromSweep :type Boolean) (SweepResult :type Hit%20Result%20Structure%20%28by%20ref%29))
  ;[1 1 1] Camera Shot Hit
  (Utilities|Casting|CastToFirstPersonProjectile OtherActor)
  (Actor|DestroyActor))

(event OnSeePawn(PawnSensing)
  (params (Pawn :type Pawn%20Object%20Reference))
  (Development|PrintString (Utilities|GetDisplayName Pawn)))

(event OnPerceptionUpdated(AIPerception)
  (params (UpdatedActors :type Array%20of%20Actor%20Object%20References)))

(event Custom|EnemyVisible
  (bind _sphere (Variables|Default|GetSphere))
  ;[1 1 1] Enemy Visibility
  (bind _asplayer (Utilities|Casting|CastToPlayer (Game|GetPlayerCharacter 0)))
  (if (Variables|/Game/Hotel/Blueprints/Player/Player.Player_C|GetCamUp _asplayer)
    (Rendering|SetVisibility _sphere false true)
    (else
      (Rendering|SetVisibility _sphere true true))))

(event Custom|Within%20Spook%20Range
  (bind _returnvalue (Game|GetPlayerCharacter 0))
  (bind _returnvalue_2 (Transformation|GetActorLocation))
  (bind _returnvalue_3 (Transformation|GetActorLocation _returnvalue))
  (bind _returnvalue_4 (- _returnvalue_2 _returnvalue_3))
  (bind _returnvalue_5 (Math|Vector|VectorLength _returnvalue_4))
  ;[1 1 1] Within Spook Range
  (if (<= _returnvalue_5 7.5e+02)
    (bind _asplayer (Utilities|Casting|CastToPlayer _returnvalue))
    (Variables|/Game/Hotel/Blueprints/Player/Player.Player_C|SetSpookLevel _asplayer (+ (Variables|/Game/Hotel/Blueprints/Player/Player.Player_C|GetSpookLevel _asplayer) (/ 1.0 _returnvalue_5)))))

(event Custom|On%20Death
  ;[1 1 1] Begin Play (Bind On Death)
  (bind _asplayer (Utilities|Casting|CastToPlayer (Game|GetPlayerCharacter 0)))
  (Default|StopHeartbeat _asplayer))

(event EventTick
  (params (DeltaSeconds :type Float%20%28single-precision%29))
  ;[1 1 1] Event Tick
  (CallFunction|EnemyVisible)
  (CallFunction|WithinSpookRange))

(event EventBeginPlay
  ;[1 1 1] Begin Play (Bind On Death)
  (EventDispatchers|BindEventtoOnDestroyed (delegate Custom|On%20Death)))

(fn ConstructionScript)