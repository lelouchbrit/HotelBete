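; Ghost enemy that spooks the player and is destroyed when a FirstPersonProjectile overlaps its CamTarget, stopping the player's heartbeat.
; Each tick it hides its sphere while the player's camera is up and, within range, raises SpookLevel by inverse distance.
; On BeginPlay it derives GhostMode from the display name of its overlapping GhostRoomBoundary, destroying itself on an unknown name.
; Movement and AI are empty stubs.
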(event OnComponentBeginOverlap(CamTarget)
  (params (OtherActor :type Actor%20Object%20Reference) (OtherComp :type Primitive%20Component%20Object%20Reference) (OtherBodyIndex :type Integer) (bFromSweep :type Boolean) (SweepResult :type Hit%20Result%20Structure%20%28by%20ref%29))
  ;[1 1 1] Camera Shot Hit
  (Utilities|Casting|CastToFirstPersonProjectile OtherActor)
  (Actor|DestroyActor))

(event Custom|EnemyVisible
  (bind _sphere (Variables|Default|GetSphere))
  ;[1 1 1] Enemy Visibility
  (bind _asplayer (Utilities|Casting|CastToPlayer (Game|GetPlayerCharacter 0)))
  (if (Variables|/Game/Hotel/Blueprints/Player/Player.Player_C|GetCamUp _asplayer)
    (Rendering|SetVisibility _sphere false true)
    (else
      (Rendering|SetVisibility _sphere true true))))

(event Custom|Within%20Spook%20Range
  (bind _returnvalue (Game|GetPlayerCharacter 0))
  (bind _returnvalue_2 (Transformation|GetActorLocation))
  (bind _returnvalue_3 (Transformation|GetActorLocation _returnvalue))
  (bind _returnvalue_4 (- _returnvalue_2 _returnvalue_3))
  (bind _returnvalue_5 (Math|Vector|VectorLength _returnvalue_4))
  ;[1 1 1] Within Spook Range
  (if (<= _returnvalue_5 7.5e+02)
    (bind _asplayer (Utilities|Casting|CastToPlayer _returnvalue))
    (Variables|/Game/Hotel/Blueprints/Player/Player.Player_C|SetSpookLevel _asplayer (+ (Variables|/Game/Hotel/Blueprints/Player/Player.Player_C|GetSpookLevel _asplayer) (/ 1.0 _returnvalue_5)))))

(event Custom|On%20Death
  ;[1 1 1] On Death
  (bind _asplayer (Utilities|Casting|CastToPlayer (Game|GetPlayerCharacter 0)))
  (Default|StopHeartbeat _asplayer))

(event EventTick
  (params (DeltaSeconds :type Float%20%28single-precision%29))
  ;[1 1 1] Event Tick
  (CallFunction|EnemyVisible)
  (CallFunction|WithinSpookRange)
  (CallFunction|AI))

(event EventBeginPlay
  ;[1 1 1] Begin Play
  ;[1 1 1] On Death
  (EventDispatchers|BindEventtoOnDestroyed (delegate Custom|On%20Death))
  ;[1 1 1] Sense BA
  (for _array_element (Collision|GetOverlappingActors (Variables|Default|GetCamTarget) "/Game/Hotel/Blueprints/Enemies/GhostRoomBoundary.GhostRoomBoundary_C" :!class /Script/Engine.PrimitiveComponent)
    (bind _asghost_room_boundary (Utilities|Casting|CastToGhostRoomBoundary _array_element))
    (Variables|Default|SetGhostBA _asghost_room_boundary)
    ;[1 1 1] Sense Mode
    (CallFunction|SenseMode)))

(fn ConstructionScript)

(fn Movement)

(fn SenseMode
  (switch string (Utilities|GetDisplayName (Variables|Default|GetGhostBA))
    (:Default
      (Development|PrintString "Error 103: Ghost Sense Mode switch statement invalid. Destroying Actor." false true "(R=0.000000,G=0.660000,B=1.000000,A=1.000000)" 1e+01)
      (Actor|DestroyActor))
    (:GhostRoom1
      (Variables|Default|SetGhostMode 1))
    (:GhostRoom2
      (Variables|Default|SetGhostMode 2))
    (:GhostRoom3
      (Variables|Default|SetGhostMode 3))
    (:GhostRoom4
      (Variables|Default|SetGhostMode 4))
    (:GhostRoom5
      (Variables|Default|SetGhostMode 5))
    (:GhostRoom6
      (Variables|Default|SetGhostMode 6))))

(fn AI)